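; BP_ConveyorT1 is a tier 1 conveyor building that carries items along its Arrow direction.
; Each Tick it offsets every actor overlapping its Box that has the "movable" tag, scaled by Speed and DeltaSeconds, without sweeping.
; Interact looks up the ItemDataComponent's data table row and returns its name, class, buy and sell values, plus the interaction widget.
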(event `self.ReceiveBeginPlay`)

(event `self.ReceiveTick`
  (params (DeltaSeconds :type "Float (single-precision)"))
  (for _array_element (`PrimitiveComponent.GetOverlappingActors` (`self.Box`) null)
    (if (`self.ActorHasTag` _array_element "movable")
      (`self.K2_AddActorWorldOffset` _array_element (* (* DeltaSeconds (`self.speed`)) (`KismetMathLibrary.GetForwardVector` (`SceneComponent.K2_GetComponentRotation` (`self.Arrow`)))) false false))))

(fn `Interact`
  (returns (ItemName :type Text) (ClassReferenceToItem :type "Actor Class Reference") (ItemCost :type "Float (double-precision)") (ItemSellValue :type "Float (double-precision)") (InteractionWidget :type "Widget Object Reference"))
  (bind (_itemid_datatable _itemid_rowname) (break `DataTableRowHandle` (`/Game/Inventory/ItemDataComponent.ItemID` (`self.ItemDataComponent`))))
  (bind _returnvalue (`|GetDataTableRow` _itemid_datatable _itemid_rowname)
    (:`then`
      (bind (_itemname _itemdescription _itemthumbnail _itemclass _itembuyvalue _itemsellvalue) (break `/Game/Inventory/fItemStruct` _returnvalue))
      (return _itemname _itemclass _itembuyvalue _itemsellvalue (`WidgetComponent.GetWidget` (`self.ItemInteractionWidget`))))))

(fn `UserConstructionScript`)