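; Base dropper building that spawns items and exposes its shop data when interacted with.
; Every tick it passes DropCube to the ACDropping component's DropItem, leaving the drop logic to that component.
; Interact looks up the ItemDataComponent's data table row and, when found, returns the item's name, class, buy and sell values, along with its interaction widget.
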(event `self.ReceiveTick`
  (params (DeltaSeconds :type "Float (single-precision)"))
  (`/Game/GameObjects/Components/AC_Dropping.DropItem` (`self.AC_Dropping`) (`self.dropCube`)))

(fn `Interact`
  (returns (ItemName :type Text) (ClassReferenceToItem :type "Actor Class Reference") (ItemCost :type "Float (double-precision)") (ItemSellValue :type "Float (double-precision)") (InteractionWidget :type "Widget Object Reference"))
  (bind (_itemid_datatable _itemid_rowname) (break `DataTableRowHandle` (`/Game/Inventory/ItemDataComponent.ItemID` (`self.ItemDataComponent`))))
  (bind _returnvalue (`|GetDataTableRow` _itemid_datatable _itemid_rowname)
    (:`then`
      (bind (_itemname _itemdescription _itemthumbnail _itemclass _itembuyvalue _itemsellvalue) (break `/Game/DataTables/fItemStruct` _returnvalue))
      (return _itemname _itemclass _itembuyvalue _itemsellvalue (`WidgetComponent.GetWidget` (`self.ItemInteractionWidget`))))))

(fn `UserConstructionScript`)