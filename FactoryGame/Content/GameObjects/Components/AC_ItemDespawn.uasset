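; AC_ItemDespawn is an actor component that destroys its owning dropped item once a despawn time has elapsed.
; On BeginPlay it reads DroppedItemDespawnTime from DT_ItemDropperData using the DropperID row.
; Tick accumulates world delta seconds until that time is exceeded, then destroys the owner and decrements WorldItemAmount on the player's BP_ThirdPersonCharacter.
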(event `self.ReceiveBeginPlay`
  (bind (_dropperid_datatable _dropperid_rowname) (break `DataTableRowHandle` (`self.dropperID`)))
  (bind _returnvalue (`|GetDataTableRow` "/Game/DropperSystem/DT_ItemDropperData.DT_ItemDropperData" _dropperid_rowname)
    (:`then`
      (set `self.Dropped Item Despawn Time` (`.DroppedItemDespawnTime_9_28DC7EAA44B9341085A23E8D47E8666E` (break `/Game/DropperSystem/fDropperStruct` _returnvalue))))))

(event `self.ReceiveTick`
  (params (DeltaSeconds :type "Float (single-precision)"))
  (if (<= (`self.despawnTimer`) (`self.Dropped Item Despawn Time`))
    (set `self.despawnTimer` (+ (`self.despawnTimer`) (`GameplayStatics.GetWorldDeltaSeconds`)))
    (else
      (`Actor.K2_DestroyActor` (`self.GetOwner`))
      (bind _asbp_third_person_character (cast `/Game/ThirdPerson/Blueprints/BP_ThirdPersonCharacter` (`GameplayStatics.GetPlayerCharacter` 0)))
      (set `/Game/ThirdPerson/Blueprints/BP_ThirdPersonCharacter.worldItemAmount` (- (`/Game/ThirdPerson/Blueprints/BP_ThirdPersonCharacter.worldItemAmount` _asbp_third_person_character) 1) _asbp_third_person_character))))