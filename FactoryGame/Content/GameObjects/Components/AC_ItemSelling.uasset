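; AC_ItemSelling is an actor component that turns its owner into a sell zone for dropped items.
; Each tick it scans actors overlapping the owner for the itemDrop tag.
; For each match it calls AddCurrency on the player character's AC_Currency, currently with a zero amount, then destroys the item through its AC_ItemDespawn component.
; The SellItem function is an empty stub.
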(event `self.ReceiveTick`
  (params (DeltaSeconds :type "Float (single-precision)"))
  (for _array_element (`Actor.GetOverlappingActors` (`self.GetOwner`) null)
    (if (`Actor.ActorHasTag` _array_element "itemDrop")
      (bind _asbp_third_person_character (cast `/Game/ThirdPerson/Blueprints/BP_ThirdPersonCharacter` (`GameplayStatics.GetPlayerCharacter` 0)))
      (`/Game/GameObjects/Components/AC_Currency.addCurrency` (`/Game/ThirdPerson/Blueprints/BP_ThirdPersonCharacter.AC_Currency` _asbp_third_person_character) 0.0)
      (`/Game/GameObjects/Components/AC_ItemDespawn.destroyItem` (`Actor.GetComponentByClass` _array_element "/Game/GameObjects/Components/AC_ItemDespawn.AC_ItemDespawn_C")))))

(fn `sellItem`)