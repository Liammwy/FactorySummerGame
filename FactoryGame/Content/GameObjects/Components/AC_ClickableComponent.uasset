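; Actor component that makes its owner clickable, highlighting it on hover and opening an item interaction menu on click.
; On BeginPlay it binds the owner's click and cursor-over events, using custom depth on the static mesh for the highlight.
; Outside the player's placement mode, every other click fills WB_ItemInteractionMenu with pickup, buy and sell text and item data.
; InPlacementMode clears the highlight and destroys the component.
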(event `self.ReceiveBeginPlay`
  (bind _returnvalue (`self.GetOwner`))
  (bind _returnvalue_2 (`Actor.GetComponentByClass` _returnvalue "/Script/Engine.StaticMeshComponent"))
  (add `Actor.OnClicked` _returnvalue (delegate `OnMouseClicked`))
  (`/Engine/EditorBlueprintResources/StandardMacros.IsValid` _returnvalue_2
    (:`Is Valid`
      (set `self.staticMeshRef` _returnvalue_2)
      (add `Actor.OnBeginCursorOver` (`self.GetOwner`) (delegate `OnMouseHover`))
      (add `Actor.OnEndCursorOver` (`self.GetOwner`) (delegate `OnMouseUnhover`)))))

(event `OnMouseHover`
  (params (TouchedActor :type "Actor Object Reference"))
  (bind _asbp_third_person_character (cast `/Game/ThirdPerson/Blueprints/BP_ThirdPersonCharacter` (`GameplayStatics.GetPlayerCharacter` 0)))
  (if (not (`/Game/ThirdPerson/Blueprints/BP_ThirdPersonCharacter.PlacementModeEnabled` _asbp_third_person_character))
    (`PrimitiveComponent.SetRenderCustomDepth` (`self.staticMeshRef`) true)))

(event `OnMouseUnhover`
  (params (TouchedActor :type "Actor Object Reference"))
  (`PrimitiveComponent.SetRenderCustomDepth` (`self.staticMeshRef`) false))

(event `OnMouseClicked`
  (params (TouchedActor :type "Actor Object Reference") (ButtonPressed :type "Key Structure" :default "None"))
  (bind _as_wb_item_interaction_menu (`self.As WB Item Interaction Menu`))
  (bind _returnvalue (`Actor.GetComponentByClass` (`self.actorHit`) "/Game/Inventory/ItemDataComponent.ItemDataComponent_C"))
  (bind (_itemid_datatable _itemid_rowname) (break `DataTableRowHandle` (`/Game/Inventory/ItemDataComponent.ItemID` _returnvalue)))
  (set `self.actorHit` TouchedActor)
  (set `self.isClicked` (not (`self.isClicked`)))
  (`/Engine/EditorBlueprintResources/StandardMacros.IsValid` (`self.staticMeshRef`)
    (:`Is Valid`
      (if (`self.isClicked`)
        (bind _asbp_third_person_character (cast `/Game/ThirdPerson/Blueprints/BP_ThirdPersonCharacter` (`GameplayStatics.GetPlayerCharacter` 0)))
        (if (not (`/Game/ThirdPerson/Blueprints/BP_ThirdPersonCharacter.PlacementModeEnabled` _asbp_third_person_character))
          (bind (_itemname _classreferencetoitem _itemcost _itemsellvalue _interactionwidget) (message `/Game/Inventory/i_InteractInterface.Interact` (`self.actorHit`)))
          (set `self.Item Name` _itemname)
          (set `self.Item Cost` _itemcost)
          (set `self.Item Sell Value` _itemsellvalue)
          (bind _output_get (set `self.Interaction Widget` _interactionwidget))
          (`Widget.SetVisibility` _output_get "Visible")
          (bind _aswb_item_interaction_menu (cast `/Game/GameObjects/UI/WB_ItemInteractionMenu` _output_get))
          (set `self.As WB Item Interaction Menu` _aswb_item_interaction_menu)
          (set `TextBlock.Text` (`|FormatText` "Pickup {0}" (`self.Item Name`)) (`/Game/GameObjects/UI/WB_ItemInteractionMenu.pickupText` (`self.As WB Item Interaction Menu`)))
          (set `TextBlock.Text` (`|FormatText` "Buy ${0}" (`self.Item Cost`)) (`/Game/GameObjects/UI/WB_ItemInteractionMenu.buyText` (`self.As WB Item Interaction Menu`)))
          (set `TextBlock.Text` (`|FormatText` "Sell ${0}" (`self.Item Sell Value`)) (`/Game/GameObjects/UI/WB_ItemInteractionMenu.sellText` (`self.As WB Item Interaction Menu`)))
          (set `/Game/GameObjects/UI/WB_ItemInteractionMenu.itemID` _itemid_rowname _as_wb_item_interaction_menu)
          (set `/Game/GameObjects/UI/WB_ItemInteractionMenu.quantity` (`/Game/Inventory/ItemDataComponent.ItemAmount` _returnvalue) _as_wb_item_interaction_menu)
          (set `/Game/GameObjects/UI/WB_ItemInteractionMenu.itemToDelete` (`self.actorHit`) _as_wb_item_interaction_menu))))))

(event `InPlacementMode`
  (`PrimitiveComponent.SetRenderCustomDepth` (`self.staticMeshRef`) false)
  (`self.K2_DestroyComponent`))