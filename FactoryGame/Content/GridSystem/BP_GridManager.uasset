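; BP_GridManager is a grid manager that spawns a square grid of BP_GridCell actors centred on the world origin at BeginPlay.
; Cells are stored row by row in GridArray, then linked to north, south, east and west neighbours using index arithmetic with edge checks.
; Lookup functions linearly search for the closest cell position or cell, with the cell search seeding its distance threshold from the world origin.
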(event `self.ReceiveBeginPlay`
  (`self.PopulateGrid`)
  (`self.PopulateNeighbours`))

(fn `GetClosestGridCell`
  (params (InPosition :type "Vector Structure"))
  (returns (OutputCell :type "/Game/GridSystem/BP_GridCell Object Reference"))
  (locals (closestDistance :type "Float (double-precision)") (startPosition :type "Vector Structure") (ArrayIndex :type Integer))
  (set `local.startPosition` InPosition)
  (set `local.closestDistance` (`KismetMathLibrary.Vector_Distance` (0.0 0.0 0.0) (`local.startPosition`)))
  (for (_array_element _array_index) (`self.gridArray`)
    (bind _returnvalue (`KismetMathLibrary.Vector_Distance` (`self.K2_GetActorLocation` _array_element) (`local.startPosition`)))
    (if (< _returnvalue (`local.closestDistance`))
      (set `local.ArrayIndex` _array_index)
      (set `local.closestDistance` _returnvalue)))
  (return (`|GetArrayItem` (`self.gridArray`) (`local.ArrayIndex`))))

(fn `GetClosestGridPosition`
  (params (InPosition :type "Vector Structure"))
  (returns (OutPosition :type "Vector Structure"))
  (locals (closestPositon :type "Vector Structure") (closestDistance :type "Float (double-precision)") (startPosition :type "Vector Structure"))
  (set `local.startPosition` InPosition)
  (bind _output_get (set `local.closestPositon` (`self.K2_GetActorLocation` (`|GetArrayItem` (`self.gridArray`)))))
  (set `local.closestDistance` (`KismetMathLibrary.Vector_Distance` _output_get (`local.startPosition`)))
  (for _array_element (`self.gridArray`)
    (bind _returnvalue (`self.K2_GetActorLocation` _array_element))
    (bind _returnvalue_2 (`KismetMathLibrary.Vector_Distance` _returnvalue (`local.startPosition`)))
    (if (< _returnvalue_2 (`local.closestDistance`))
      (set `local.closestPositon` _returnvalue)
      (set `local.closestDistance` _returnvalue_2)))
  (return (`local.closestPositon`)))

(fn `PopulateGrid`
  (locals (worldOffset :type "Float (double-precision)"))
  (bind _worldgridsize (`self.worldGridSize`))
  (bind _worldgridsize_2 (`self.worldGridSize`))
  (bind _worldoffset (`local.worldOffset`))
  (`KismetArrayLibrary.Array_Clear` (`self.gridArray`))
  (set `local.worldOffset` (- (* (* (`self.gridSize`) _worldgridsize) 0.5) (* _worldgridsize 0.5)))
  (for _index (range (`self.gridSize`))
    (for _index_2 (range (`self.gridSize`))
      (bind _returnvalue (`|SpawnActorFromClass` "/Game/GridSystem/BP_GridCell.BP_GridCell_C" (`KismetMathLibrary.MakeTransform` (`KismetMathLibrary.MakeVector` (- (* _index_2 _worldgridsize_2) _worldoffset) (- (* _worldgridsize_2 _index) _worldoffset))) "AlwaysSpawn" "MultiplyWithRoot" null null))
      (`KismetArrayLibrary.Array_Add` (`self.gridArray`) _returnvalue))))

(fn `PopulateNeighbours`
  (locals (localArrayINDX :type Integer))
  (bind _returnvalue (+ (`local.localArrayINDX`) (`self.gridSize`)))
  (for (_array_element _array_index) (`self.gridArray`)
    ;[1 1 1] South Neighbour
    (bind _output_get (set `local.localArrayINDX` _array_index))
    (bind _returnvalue_2 (- _output_get (`self.gridSize`)))
    (if (>= _returnvalue_2 0)
      (set `/Game/GridSystem/BP_GridCell.NeighbourSouth` (`|GetArrayItem` (`self.gridArray`) _returnvalue_2) _array_element))
    ;[1 1 1] Noth Neighbour
    (if (< _returnvalue (`KismetArrayLibrary.Array_Length` (`self.gridArray`)))
      (set `/Game/GridSystem/BP_GridCell.NeighbourNorth` (`|GetArrayItem` (`self.gridArray`) _returnvalue) _array_element))
    ;[1 1 1] West Neighbour
    (if (not (or (== (`local.localArrayINDX`) 0) (== (mod (`local.localArrayINDX`) (`self.gridSize`)) 0)))
      (set `/Game/GridSystem/BP_GridCell.NeighbourWest` (`|GetArrayItem` (`self.gridArray`) (- (`local.localArrayINDX`) 1)) _array_element))
    ;[1 1 1] East Neighbour
    (if (not (== (mod (+ (`local.localArrayINDX`) 1) (`self.gridSize`)) 0))
      (set `/Game/GridSystem/BP_GridCell.NeighbourEast` (`|GetArrayItem` (`self.gridArray`) (+ (`local.localArrayINDX`) 1)) _array_element))))

(fn `UserConstructionScript`)