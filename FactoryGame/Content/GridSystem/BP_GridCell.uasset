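; BP_GridCell is a single cell in the grid system that tracks what is built on it.
; SetOccupied stores the build type and occupying actor and flags the cell as occupied, unless the type is the zero value, which marks it free.
; It references north, east, south and west neighbours, used here only by unconnected debug calls to an event that changes a cell's sphere material.
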(event `SetOccupied`
  (params (NewBuildType :type "/Game/GridSystem/BuildingTypeEnum Enum" :default "NewEnumerator3") (NewOccupyingActor :type "Actor Object Reference"))
  (set `self.IsOccupied` true)
  (set `self.OccupyingType` NewBuildType)
  (set `self.OccupyingActor` NewOccupyingActor)
  (if (== (`self.OccupyingType`) 0)
    (set `self.IsOccupied` false)))

(event `DebugShowNeighbourOccupied`
  (`PrimitiveComponent.SetMaterial` (`self.Sphere`) 0 "/Game/StarterContent/Materials/M_Brick_Cut_Stone.M_Brick_Cut_Stone"))

(fn `UserConstructionScript`)